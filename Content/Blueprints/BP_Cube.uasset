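; BP_Cube displays an actor above its cube, chosen by its current InputValue.
; Tick polls InputValue against StoreValue and calls ValueChanged when they differ.
; ValueChanged destroys the previous actor, scans every DT_Meshes row for a matching Value and spawns that row's actor class.
; The SlimeMotion timeline then animates the spawned actor's uniform scale, multiplied by Size.
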(event Custom|ValueChanged
  (Utilities|IsValid (Variables|Default|GetSpawned)
    (:Is%20Valid
      (Actor|DestroyActor (Variables|Default|GetSpawned)))
    (:Is%20Not%20Valid
      _))
  (bind _outrownames (DataTable|GetDataTableRowNames "/Game/DataTable/DT_Meshes.DT_Meshes"))
  (for _array_element _outrownames
    (bind _returnvalue (Utilities|GetDataTableRow "/Game/DataTable/DT_Meshes.DT_Meshes" _array_element)
      (:then
        (if (== (Variables|Default|GetInputValue) (.value (Utilities|Struct|BreakST_Meshes _returnvalue)))
          (bind _returnvalue_2 (Game|SpawnActorfromClass (.Actor (Utilities|Struct|BreakST_Meshes _returnvalue)) (Math|Transform|MakeTransform (+ (Transformation|GetWorldLocation (Variables|Default|GetCube)) "0.000000,0.000000,100.000000") "0, 0, 0" (Math|Vector|MakeVector 0.5 0.5 0.5)) "Undefined" "MultiplyWithRoot" 0 0))
          (bind _output_get (Variables|Default|SetSpawned _returnvalue_2))
          (Utilities|IsValid _output_get
            (:Is%20Valid
              (bind _newtrack_0 (Timeline|SlimeMotion PlayFromStart)
                (:Update
                  (Transformation|SetActorScale3D _output_get (Math|Vector|MakeVector (* _newtrack_0 (Variables|Default|GetSize)) (* _newtrack_0 (Variables|Default|GetSize)) (* _newtrack_0 (Variables|Default|GetSize)))))))
            (:Is%20Not%20Valid
              (Timeline|SlimeMotion Stop))))))))

(event EventBeginPlay)

(event Collision|EventActorBeginOverlap
  (params (OtherActor :type Actor%20Object%20Reference)))

(event EventTick
  (params (DeltaSeconds :type Float%20%28single-precision%29))
  (if (!= (Variables|Default|GetInputValue) (Variables|Default|GetStoreValue))
    (CallFunction|ValueChanged)
    (Variables|Default|SetStoreValue (Variables|Default|GetInputValue))))

(fn ConstructionScript)