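; Spawner actor that creates a stack of instanced static meshes and slides them along local X at individual speeds.
; The construction script adds the instances at random X positions, spaced by Offset in Z, storing each index and a random speed in parallel arrays.
; Tick moves each stored instance with index below 10 by its speed times delta time, updating transforms within a single InstancedStaticMesh component.
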(event EventBeginPlay)

(event EventTick
  (params (DeltaSeconds :type Float%20%28single-precision%29))
  (bind _instancedstaticmesh (Variables|Default|GetInstancedStaticMesh))
  (for _array_element (Variables|Default|GetInstances)
    (if (< _array_element 10)
      (Components|InstancedStaticMesh|UpdateInstanceTransform _instancedstaticmesh _array_element (Math|Transform|MakeTransform (+ (.location (.OutInstanceTransform (Components|InstancedStaticMesh|GetInstanceTransform _instancedstaticmesh _array_element false))) (Math|Vector|MakeVector (* DeltaSeconds (Utilities|Array|Get(acopy) (Variables|Default|GetFloats) _array_element)) 0.0 0.0)) "0, 0, 0" (.scale (.OutInstanceTransform (Components|InstancedStaticMesh|GetInstanceTransform _instancedstaticmesh _array_element false)))) false true false))))

(fn ConstructionScript
  (for _index (range 0 10)
    (bind _returnvalue (Components|InstancedStaticMesh|AddInstance (Variables|Default|GetInstancedStaticMesh) (Math|Transform|MakeTransform (Math|Vector|MakeVector (Math|Random|RandomFloatinRange 1e+02 1e+03) 0.0 (* _index (Variables|Default|GetOffset))) "0, 0, 0" "5.000000,5.000000,5.000000") false))
    (Utilities|Array|Add (Variables|Default|GetInstances) _returnvalue)
    (Development|PrintString (Utilities|String|ToString(Integer) _returnvalue))
    (Utilities|Array|Add (Variables|Default|GetFloats) (Math|Random|RandomFloatinRange 1e+02 2e+02))))