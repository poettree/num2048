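; BP_Planet is a solar system planet actor whose sphere orbits and spins, using data looked up by PlanetName in DT_Solar_System_Planets.
; BeginPlay sets the sphere's size from scaled, clamped diameter.
; Tick accumulates time to place it on a sine/cosine circle of clamped distance, with axial tilt and spin scaled by RotationPeriod.
; Orbit rate ignores RevolutionPeriod, completing one lap per second; the RotatingMovement logic using it never runs.
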(event EventBeginPlay
  (bind _returnvalue (Utilities|GetDataTableRow "/Game/Assets/SolarSystem/DT_Solar_System_Planets.DT_Solar_System_Planets" (Variables|Default|GetPlanetName))
    (:then
      (Transformation|SetRelativeTransform (Variables|Default|GetSphere) (Math|Transform|MakeTransform (Math|Vector|MakeVector 0.0 0.0 0.0) "0, 0, 0" (* "1.000000,1.000000,1.000000" (Math|Float|Clamp(Float) (* (.Diameter (Utilities|Struct|BreakST_SolarSystem _returnvalue)) (Variables|Scaling|GetDiameterScale)) 1.5 2.5))) false false))))

(event Collision|EventActorBeginOverlap
  (params (OtherActor :type Actor%20Object%20Reference)))

(event EventTick
  (params (DeltaSeconds :type Float%20%28single-precision%29))
  (bind _output_get (Variables|Default|SetStackedRotation (+ (Variables|Default|GetStackedRotation) DeltaSeconds)))
  (Variables|Default|Setangle (* (* (Math|Trig|GetPI) 2.0) _output_get))
  (Transformation|SetRelativeTransform (Variables|Default|GetSphere) (Math|Transform|MakeTransform (* (Math|Vector|MakeVector (Math|Trig|Sin(Radians) (Variables|Default|Getangle)) (Math|Trig|Cos(Radians) (Variables|Default|Getangle)) 0.0) (Math|Float|Clamp(Float) (* (.Distance (Utilities|Struct|BreakST_SolarSystem (stale EventBeginPlay _returnvalue))) (Variables|Scaling|GetDistanceScale)) 0.1 8e+01)) (Math|Rotator|MakeRotator (.AxialTilt (Utilities|Struct|BreakST_SolarSystem (stale EventBeginPlay _returnvalue))) 0.0 (* _output_get (* (.RotationPeriod (Utilities|Struct|BreakST_SolarSystem (stale EventBeginPlay _returnvalue))) (Variables|Scaling|GetRotationScale)))) (* "1.000000,1.000000,1.000000" (Math|Float|Clamp(Float) (* (.Diameter (Utilities|Struct|BreakST_SolarSystem (stale EventBeginPlay _returnvalue))) (Variables|Scaling|GetDiameterScale)) 1.5 2.5))) false false))

(fn ConstructionScript)

(fn GetCircle)